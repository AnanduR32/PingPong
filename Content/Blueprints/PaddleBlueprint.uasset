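; Player-controlled paddle pawn for a ping pong game that slides along its Y axis.
; BeginPlay registers the ping pong Enhanced Input mapping context with the player controller, then creates the score widget and adds it to the viewport as the HUD.
; MoveAction offsets the Cube component by input times PlayerSpeed, with sweep for collision and no delta-time scaling.
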(event `self.ReceiveBeginPlay`
  (bind _asplayer_controller (cast `PlayerController` (`self.GetController`)))
  (bind _returnvalue (pcsubsystem `EnhancedInputLocalPlayerSubsystem` _asplayer_controller))
  (`/Engine/EditorBlueprintResources/StandardMacros.IsValid` _returnvalue
    (:`Is Valid`
      (`EnhancedInputSubsystemInterface.AddMappingContext` _returnvalue "/Game/Controls/PingPongInputMappingContext.PingPongInputMappingContext" 0 (struct))
      (bind _returnvalue_2 (`|CreateWidget` "/Game/Blueprints/ScoreWidgetBP.ScoreWidgetBP_C"))
      (bind _output_get (set `self.ScoreHUD` _returnvalue_2))
      (`UserWidget.AddToViewport` _output_get 0))))

(event `EnhancedInput|/Game/Controls/MoveAction`
  (params (ActionValue :type "Float (double-precision)") (ElapsedSeconds :type "Float (double-precision)") (TriggeredSeconds :type "Float (double-precision)") (InputAction :type "InputAction Object Reference" :default "/Game/Controls/MoveAction.MoveAction"))
  (:`Triggered`
    (`SceneComponent.K2_AddLocalOffset` (`self.Cube`) (`KismetMathLibrary.MakeVector` 0.0 (* ActionValue (`self.PlayerSpeed`))) true false)))

(fn `UserConstructionScript`)