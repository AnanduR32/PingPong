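; Physics-driven ball actor that speeds up with each hit and triggers a replacement spawn when destroyed.
; On BeginPlay it registers itself with the AI actor and launches its sphere along X, with a flag choosing the direction.
; Each hit raises the speed, re-applies it along the current velocity direction clamped between min and max, and prints the result.
; On destruction it calls SpawnBall on its spawner reference.
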(event `self.ReceiveBeginPlay`
  (bind _returnvalue (`GameplayStatics.GetActorOfClass` "/Game/Blueprints/AI.AI_C"))
  (bind _output_get (set `self.AI Ref` _returnvalue))
  (set `/Game/Blueprints/AI.BallRef` self _output_get)
  (`PrimitiveComponent.AddImpulse` (`self.Sphere`) (`KismetMathLibrary.MakeVector` (* (`self.InitialImpulseOnSpawn`) (`KismetMathLibrary.SelectFloat` 1.0 -1.0 (`self.doSwitch`)))) "None" true))

(event `self.ReceiveHit`
  (params (MyComp :type "PrimitiveComponent Object Reference") (Other :type "Actor Object Reference") (OtherComp :type "PrimitiveComponent Object Reference") (bSelfMoved :type Boolean) (HitLocation :type "Vector Structure") (HitNormal :type "Vector Structure") (NormalImpulse :type "Vector Structure") (Hit :type "HitResult Structure (by ref)"))
  (bind _sphere (`self.Sphere`))
  (bind _output_get (set `self.BallSpeed` (+ (`self.BallSpeed`) 30.0)))
  (bind _returnvalue (`PrimitiveComponent.GetPhysicsLinearVelocity` _sphere "None"))
  (`PrimitiveComponent.SetPhysicsLinearVelocity` _sphere (`KismetMathLibrary.ClampVectorSize` (* (`KismetMathLibrary.Normal` _returnvalue) _output_get) (`self.BallSpeedMin`) (`self.BallSpeedMax`)) false "None")
  (bind _returnvalue_2 (`PrimitiveComponent.GetPhysicsLinearVelocity` _sphere "None"))
  (`KismetSystemLibrary.PrintString` (`KismetStringLibrary.Conv_VectorToString` _returnvalue_2)))

(event `self.ReceiveDestroyed`
  (`/Game/Blueprints/BallSpawnerBP.Spawn Ball` (`self.BallSpawnRef`)))

(fn `UserConstructionScript`)