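; GoalBP is a goal trigger that awards a point when a ball enters its box.
; On BeginPlay it caches the player's paddle pawn to reach that paddle's ScoreHUD.
; An overlapping BallBlueprint is destroyed, then the HasPlayerScored flag selects whether the player's or the AI's score updates, letting one class serve either side.
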(event `self.ReceiveBeginPlay`
  (bind _aspaddle_blueprint (cast `/Game/Blueprints/PaddleBlueprint` (`GameplayStatics.GetPlayerPawn` 0)))
  (set `self.PaddleRef` _aspaddle_blueprint))

(event `self.Box.OnComponentBeginOverlap`
  (params (OverlappedComponent :type "PrimitiveComponent Object Reference") (OtherActor :type "Actor Object Reference") (OtherComp :type "PrimitiveComponent Object Reference") (OtherBodyIndex :type Integer) (bFromSweep :type Boolean) (SweepResult :type "HitResult Structure (by ref)"))
  (bind _paddleref (`self.PaddleRef`))
  (bind _asball_blueprint (cast `/Game/Blueprints/BallBlueprint` OtherActor))
  (`self.K2_DestroyActor` _asball_blueprint)
  (if (`self.hasPlayerScored`)
    (`/Game/Blueprints/ScoreWidgetBP.Update Player score` (`/Game/Blueprints/PaddleBlueprint.ScoreHUD` _paddleref))
    (else
      (`/Game/Blueprints/ScoreWidgetBP.Update Ai score` (`/Game/Blueprints/PaddleBlueprint.ScoreHUD` _paddleref)))))

(fn `UserConstructionScript`)